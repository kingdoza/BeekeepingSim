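; Comb slot actor for an uncapping table that animates its attach point when a comb is grabbed or released.
; On BeginPlay it stores the AttachComponent's relative location as the release position and derives a raised grab position along its up vector.
; The TL_GrabRelease timeline lerps the component between them, playing forward on grab and reversing on release or aborted grab.
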(event EventBeginPlay
  (bind _attachcomponent (Variables|Default|GetAttachComponent))
  (bind _output_get (Variables|Default|SetReleaseLocation (Variables|/Script/Engine.SceneComponent|GetRelativeLocation _attachcomponent)))
  (Variables|Default|SetGrabLocation (+ (* (Math|Vector|GetUpVector _attachcomponent) 55.0) _output_get)))

(event Collision|EventActorBeginOverlap
  (params (OtherActor :type Actor%20Object%20Reference)))

(event EventTick
  (params (DeltaSeconds :type Float%20%28single-precision%29)))

(event EventCombGrabbed
  (params (CombActor :type Beehive%20Comb%20Actor%20Object%20Reference) (InteractingCharacter :type Beekeeper%20Character%20Object%20Reference))
  (bind _newtrack_0 (Timeline|TL_GrabRelease Play)
    (:Update
      (Transformation|SetRelativeLocation (Variables|Default|GetAttachComponent) (Math|Vector|Lerp(Vector) (Variables|Default|GetReleaseLocation) (Variables|Default|GetGrabLocation) _newtrack_0) false false))))

(event EventCombReleased
  (params (CombActor :type Beehive%20Comb%20Actor%20Object%20Reference) (InteractingCharacter :type Beekeeper%20Character%20Object%20Reference))
  (bind _newtrack_0 (Timeline|TL_GrabRelease Reverse)
    (:Update
      (Transformation|SetRelativeLocation (Variables|Default|GetAttachComponent) (Math|Vector|Lerp(Vector) (Variables|Default|GetReleaseLocation) (Variables|Default|GetGrabLocation) _newtrack_0) false false))))

(event EventReceiveCombGrabAborted
  (params (CombActor :type Beehive%20Comb%20Actor%20Object%20Reference) (InteractingCharacter :type Beekeeper%20Character%20Object%20Reference))
  (bind _newtrack_0 (Timeline|TL_GrabRelease Reverse)
    (:Update
      (Transformation|SetRelativeLocation (Variables|Default|GetAttachComponent) (Math|Vector|Lerp(Vector) (Variables|Default|GetReleaseLocation) (Variables|Default|GetGrabLocation) _newtrack_0) false false))))

(fn ConstructionScript)