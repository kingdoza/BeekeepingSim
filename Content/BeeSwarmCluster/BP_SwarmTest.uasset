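; BP_SwarmTest is a test Blueprint that drives a Niagara swarm effect, apparently for a bee swarm cluster.
; On BeginPlay it initializes the effect's spawn amount, sphere radius and alive radius through Niagara user variables.
; Pressing the 2 key increments CurrentAliveRadius, pushes it to the AliveRadius parameter and prints the new value for debugging.
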(event EventBeginPlay
  (bind _niagara (Variables|Default|GetNiagara))
  (Class|NiagaraComponent|SetVariableInt _niagara "SpawnAmount" 200)
  (Niagara|SetNiagaraVariable(Float) _niagara "SphereRadius" 5e+01)
  (Niagara|SetNiagaraVariable(Float) _niagara "AliveRadius" 0.0))

(event Collision|EventActorBeginOverlap
  (params (OtherActor :type Actor%20Object%20Reference)))

(event EventTick
  (params (DeltaSeconds :type Float%20%28single-precision%29)))

(event Input|KeyboardEvents|2
  (params (Key :type Key%20Structure :default "None"))
  (:Pressed
    (bind _output_get (Variables|Default|SetCurrentAliveRadius (+ (Variables|Default|GetCurrentAliveRadius) 1.0)))
    (Niagara|SetNiagaraVariable(Float) (Variables|Default|GetNiagara) "AliveRadius" _output_get)
    (Development|PrintString (Utilities|String|ToString(Float) _output_get))))

(fn ConstructionScript)