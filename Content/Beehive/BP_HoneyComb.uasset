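; Honeycomb actor for the beehive that animates the comb when it is shaken or flipped.
; A shake plays a timeline that offsets the comb pivot vertically along a curve.
; A flip takes a direction, stores the current yaw, and uses a second timeline to lerp the pivot half a turn left or right.
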(event EventBeginPlay)

(event Collision|EventActorBeginOverlap
  (params (OtherActor :type Actor%20Object%20Reference)))

(event EventTick
  (params (DeltaSeconds :type Float%20%28single-precision%29)))

(event EventCombFlippedWithDirection
  (params (NewVisibleFace :type EBeehiveCombVisibleFace%20Enum :default "Front") (FlipDirection :type EBeehiveCombFlipDirection%20Enum :default "Left"))
  (bind _output_get (Variables|Default|SetFlipStartYaw (.yaw (Variables|/Script/Engine.SceneComponent|GetRelativeRotation (Variables|Default|GetCombPivotRoot)))))
  (Variables|Default|SetFlipTargetYaw (+ _output_get (Utilities|Select :Index FlipDirection :Left 1.8e+02 :Right -1.8e+02)))
  (bind _newtrack_0 (Timeline|TL_Flip PlayFromStart)
    (:Update
      (Transformation|SetRelativeRotation (Variables|Default|GetCombPivotRoot) (Math|Rotator|MakeRotator 0.0 0.0 (Math|Float|Lerp (Variables|Default|GetFlipStartYaw) (Variables|Default|GetFlipTargetYaw) _newtrack_0)) false false))))

(event EventCombShaken
  (params (StrokeCount :type Integer) (ReductionRatio :type Float%20%28single-precision%29))
  (bind _newtrack_0 (Timeline|TL_Shake PlayFromStart)
    (:Update
      (Transformation|SetRelativeLocation (Variables|Default|GetCombPivotRoot) (Math|Vector|MakeVector 0.0 0.0 (* _newtrack_0 -1.2e+02)) false false))))

(fn ConstructionScript)