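; Beehive actor Blueprint that animates the hive lid in response to part-focus interaction.
; Focus begin on the lid plays a timeline that lerps the lid mesh's relative rotation open, while cancel or abort reverses it.
; Comb focus events are empty stubs.
; Unconnected leftover nodes cover moving a comb from its slot, setting a Niagara swarm Disease parameter and printing a sanitation value.
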(event OnPartFocusBegin(LidPartFocusAction)
  (params (ActionComponent :type Cursor%20Part%20Focus%20Action%20Component%20Object%20Reference) (ScopeComponent :type Cursor%20Part%20Focus%20Scope%20Component%20Object%20Reference) (InteractingCharacter :type Beekeeper%20Character%20Object%20Reference))
  (bind _newtrack_0 (Timeline|TL_LidOpenClose Play)
    (:Update
      (Transformation|SetRelativeRotation (Variables|Default|GetLid%20Mesh) (Math|Rotator|Lerp(Rotator) "0.000000,90.000000,0.000000" "-60.000000,90.000000,0.000000" _newtrack_0) false false))))

(event OnPartFocusCancel(LidPartFocusAction)
  (params (ActionComponent :type Cursor%20Part%20Focus%20Action%20Component%20Object%20Reference) (ScopeComponent :type Cursor%20Part%20Focus%20Scope%20Component%20Object%20Reference) (InteractingCharacter :type Beekeeper%20Character%20Object%20Reference))
  (bind _newtrack_0 (Timeline|TL_LidOpenClose Reverse)
    (:Update
      (Transformation|SetRelativeRotation (Variables|Default|GetLid%20Mesh) (Math|Rotator|Lerp(Rotator) "0.000000,90.000000,0.000000" "-60.000000,90.000000,0.000000" _newtrack_0) false false))))

(event OnPartFocusAbort(LidPartFocusAction)
  (params (ActionComponent :type Cursor%20Part%20Focus%20Action%20Component%20Object%20Reference) (ScopeComponent :type Cursor%20Part%20Focus%20Scope%20Component%20Object%20Reference) (InteractingCharacter :type Beekeeper%20Character%20Object%20Reference))
  (bind _newtrack_0 (Timeline|TL_LidOpenClose Reverse)
    (:Update
      (Transformation|SetRelativeRotation (Variables|Default|GetLid%20Mesh) (Math|Rotator|Lerp(Rotator) "0.000000,90.000000,0.000000" "-60.000000,90.000000,0.000000" _newtrack_0) false false))))

(event EventBeginPlay)

(event Collision|EventActorBeginOverlap
  (params (OtherActor :type Actor%20Object%20Reference)))

(event EventTick
  (params (DeltaSeconds :type Float%20%28single-precision%29)))

(event EventCombPartFocusCancel
  (params (CombActor :type Beehive%20Comb%20Actor%20Object%20Reference) (InteractingCharacter :type Beekeeper%20Character%20Object%20Reference)))

(event EventCombPartFocusBegin
  (params (CombActor :type Beehive%20Comb%20Actor%20Object%20Reference) (InteractingCharacter :type Beekeeper%20Character%20Object%20Reference)))

(event EventOnFocusConfirm
  (params (InteractingCharacter :type Beekeeper%20Character%20Object%20Reference)))

(event EventOnFocusCancel
  (params (InteractingCharacter :type Beekeeper%20Character%20Object%20Reference)))

(event EventReceiveCombPartFocusAbort
  (params (CombActor :type Beehive%20Comb%20Actor%20Object%20Reference) (InteractingCharacter :type Beekeeper%20Character%20Object%20Reference)))

(event Input|KeyboardEvents|1
  (params (Key :type Key%20Structure)))

(fn ConstructionScript)