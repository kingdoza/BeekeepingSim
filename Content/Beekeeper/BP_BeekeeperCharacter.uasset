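; Beekeeper player character Blueprint that sets up the starting loadout and HUD on BeginPlay.
; It seeds the BeekeeperHotbar component with beekeeping tools and consumables, then creates a hidden focus blur, crosshair, focus prompt and hotbar widget fed by that component.
; BeekeeperFocus toggles the crosshair through a visibility event.
; The hotbar-changed binding and a spec-based item grant are left unconnected.
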(event Custom|OnHotbarChanged_Event
  (Default|RefreshHotbar (stale EventBeginPlay _returnvalue_5)))

(event Custom|OnCrosshairVisibilityChanged_Event
  (params (bVisible :type Boolean))
  (bind _crosshairwidget (Variables|UI|GetCrosshairWidget))
  (if bVisible
    (Widget|SetVisibility _crosshairwidget "Visible")
    (else
      (Widget|SetVisibility _crosshairwidget "Hidden"))))

(event EventBeginPlay
  (bind _returnvalue (Game|GetPlayerController 0))
  (bind _beekeeperhotbar (Variables|Default|GetBeekeeperHotbar))
  (Utilities|FlowControl|Sequence
    (:then_0
      (Class|BeekeeperHotbarComponent|TryAcquireItem _beekeeperhotbar "/Game/Items/Definitions/DA_Uncapper.DA_Uncapper" 1)
      (Class|BeekeeperHotbarComponent|TryAcquireItem _beekeeperhotbar "/Game/Items/Definitions/DA_BeeBrush.DA_BeeBrush" 1)
      (Class|BeekeeperHotbarComponent|TryAcquireItem _beekeeperhotbar "/Game/Items/Definitions/DA_PollenPatty.DA_PollenPatty" 5)
      (Class|BeekeeperHotbarComponent|TryAcquireItem _beekeeperhotbar "/Game/Items/Definitions/DA_Sprayer.DA_Sprayer" 1)
      (Class|BeekeeperHotbarComponent|TryAcquireItem _beekeeperhotbar "/Game/Items/Definitions/DA_HoneyComb.DA_HoneyComb" 2)
      (Class|BeekeeperHotbarComponent|TryAcquireItem _beekeeperhotbar "/Game/Items/Definitions/DA_Smoker.DA_Smoker" 1))
    (:then_1
      (bind _returnvalue_2 (UserInterface|CreateWidget "/Game/UI/WBP_TranslucentBlur.WBP_TranslucentBlur_C" _returnvalue))
      (bind _output_get (Variables|UI|SetFocusBlurWidget _returnvalue_2))
      (Widget|SetVisibility _output_get "Hidden")
      (UserInterface|Viewport|AddtoViewport _output_get 0)
      (bind _returnvalue_3 (UserInterface|CreateWidget "/Game/UI/WBP_Crosshair.WBP_Crosshair_C" _returnvalue))
      (bind _output_get_2 (Variables|UI|SetCrosshairWidget _returnvalue_3))
      (UserInterface|Viewport|AddtoViewport _output_get_2 0)
      (bind _returnvalue_4 (UserInterface|CreateWidget "/Game/UI/WBP_FocusPrompt.WBP_FocusPrompt_C" _returnvalue))
      (UserInterface|Viewport|AddtoViewport _returnvalue_4 0)
      (EventDispatchers|BindEventtoOnCrosshairVisibilityChanged (Variables|Default|GetBeekeeperFocus) (delegate Custom|OnCrosshairVisibilityChanged_Event))
      (bind _returnvalue_5 (UserInterface|CreateWidget "/Game/UI/WBP_Hotbar.WBP_Hotbar_C" _returnvalue (Variables|Default|GetBeekeeperHotbar)))
      (UserInterface|Viewport|AddtoViewport _returnvalue_5 0))))

(event Collision|EventActorBeginOverlap
  (params (OtherActor :type Actor%20Object%20Reference)))

(event EventTick
  (params (DeltaSeconds :type Float%20%28single-precision%29)))

(fn ConstructionScript)